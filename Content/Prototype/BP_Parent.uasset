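; BP_Parent is an inspectable object that flies from its placed transform to the first-person player's inspection point and can be returned.
; Starting inspection makes the player's capsule ignore WorldDynamic, flags the player as inspecting and disables movement.
; A timeline lerps location toward the character's Sphere and rotation toward its camera, then notifies the character when finished.
; Stopping inspection reverses the timeline back to the transform saved at BeginPlay.
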(event Custom|CustomEvent
  (bind _initialposition (Variables|Default|GetInitialPosition))
  (bind _asbp_first_person_character (Utilities|Casting|CastToBP_FirstPersonCharacter (Game|GetPlayerCharacter 0)))
  (Collision|SetCollisionResponsetoChannel (Variables|/Script/Engine.Character|GetCapsuleComponent _asbp_first_person_character) "ECC_WorldDynamic" "ECR_Ignore")
  (Variables|/Game/FirstPerson/Blueprints/BP_FirstPersonCharacter.BP_FirstPersonCharacter_C|SetIs%20Inspecting _asbp_first_person_character true)
  (Variables|/Game/FirstPerson/Blueprints/BP_FirstPersonCharacter.BP_FirstPersonCharacter_C|Setcanmove _asbp_first_person_character false)
  (bind _newtrack_0 (Timeline|Timeline Play)
    (:Update
      (Transformation|SetActorLocationAndRotation (Math|Vector|Lerp(Vector) (.location _initialposition) (Transformation|GetWorldLocation (Variables|/Game/FirstPerson/Blueprints/BP_FirstPersonCharacter.BP_FirstPersonCharacter_C|GetSphere _asbp_first_person_character)) _newtrack_0) (Math|Rotator|Lerp(Rotator) (.rotation _initialposition) (Transformation|GetWorldRotation (Variables|/Game/FirstPerson/Blueprints/BP_FirstPersonCharacter.BP_FirstPersonCharacter_C|GetFirstPersonCamera _asbp_first_person_character)) _newtrack_0)))
    (:Finished
      (Default|TimelineFinished _asbp_first_person_character))))

(event EventBeginPlay
  (Variables|Default|SetInitialPosition (Transformation|GetWorldTransform (Variables|Default|GetDefaultSceneRoot))))

(event Collision|EventActorBeginOverlap
  (params (OtherActor :type Actor%20Object%20Reference)))

(event EventTick
  (params (DeltaSeconds :type Float%20%28single-precision%29)))

(event EventStopObjetInspect
  (bind _initialposition (Variables|Default|GetInitialPosition))
  (bind _newtrack_0 (Timeline|Timeline Reverse)
    (:Update
      (Transformation|SetActorLocationAndRotation (Math|Vector|Lerp(Vector) (.location _initialposition) (Transformation|GetWorldLocation (Variables|/Game/FirstPerson/Blueprints/BP_FirstPersonCharacter.BP_FirstPersonCharacter_C|GetSphere (stale Custom|CustomEvent _asbp_first_person_character))) _newtrack_0) (Math|Rotator|Lerp(Rotator) (.rotation _initialposition) (Transformation|GetWorldRotation (Variables|/Game/FirstPerson/Blueprints/BP_FirstPersonCharacter.BP_FirstPersonCharacter_C|GetFirstPersonCamera (stale Custom|CustomEvent _asbp_first_person_character))) _newtrack_0)))
    (:Finished
      (Default|TimelineFinished (stale Custom|CustomEvent _asbp_first_person_character)))))

(fn ConstructionScript)