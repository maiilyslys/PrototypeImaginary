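; Prototype test actor that rotates itself from mouse input.
; Actor click, MouseX and MouseY events all feed one AddActorWorldRotation node, which applies doubled axis values to pitch and yaw with no roll.
; YAw and Pitch functions combine a single-axis rotator with the current rotation, YAw negating its input, but the event graph does not call them.
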(event EventTick
  (params (DeltaSeconds :type Float%20%28single-precision%29)))

(event MouseInput|EventActorOnClicked
  (params (ButtonPressed :type Key%20Structure))
  (Class|Actor|AddActorWorldRotation (Math|Rotator|MakeRotator 0.0 (* 2.0 (stale Input|MouseEvents|MouseY AxisValue)) (* (stale Input|MouseEvents|MouseX AxisValue) 2.0))))

(event Input|MouseEvents|MouseX
  (params (AxisValue :type Float%20%28single-precision%29))
  (Class|Actor|AddActorWorldRotation (Math|Rotator|MakeRotator 0.0 (* 2.0 (stale Input|MouseEvents|MouseY AxisValue)) (* AxisValue 2.0))))

(event Input|MouseEvents|MouseY
  (params (AxisValue :type Float%20%28single-precision%29))
  (Class|Actor|AddActorWorldRotation (Math|Rotator|MakeRotator 0.0 (* 2.0 AxisValue) (* (stale Input|MouseEvents|MouseX AxisValue) 2.0))))

(fn ConstructionScript)

(fn YAw
  (params (A :type Float%20%28double-precision%29))
  (Transformation|SetActorRotation (Math|Rotator|CombineRotators (Math|Rotator|MakeRotator 0.0 0.0 (* A -1.0)) (Transformation|GetActorRotation))))

(fn Pitch
  (params (Y%20%28Pitch%29 :type Float%20%28single-precision%29))
  (Transformation|SetActorRotation (Math|Rotator|CombineRotators (Math|Rotator|MakeRotator 0.0 Y%20%28Pitch%29 0.0) (Transformation|GetActorRotation))))